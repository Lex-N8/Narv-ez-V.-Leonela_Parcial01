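; BP_Enemigo_2 is an enemy actor that moves itself and can fire bullets.
; Every Tick it adds its velocity as a local offset, without sweep or delta-time scaling.
; Helper functions set movement and bullet velocities, scale a value by a multiplier, and spawn a BP_Bala at the enemy's location with a velocity.
; Nothing in this Blueprint calls these helpers.
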(event `self.ReceiveTick`
  (params (DeltaSeconds :type "Float (single-precision)"))
  (`self.K2_AddActorLocalOffset` (`self.Velocidad`)))

(fn `FloatMult`
  (params (Valor :type "Vector Structure"))
  (returns (Resultado :type "Vector Structure"))
  (return (* Valor (`self.Float Mult`))))

(fn `Setear Velocidad`
  (params (Velocidad :type "Vector Structure"))
  (set `self.Velocidad` Velocidad))

(fn `SetearVelocidadBala`
  (params (Velocidad :type "Vector Structure"))
  (set `self.Velocidad_1` Velocidad))

(fn `SpawnearBala`
  (`|SpawnActorFromClass` "/Game/BP_Bala.BP_Bala_C" (`KismetMathLibrary.MakeTransform` (`self.K2_GetActorLocation`)) "Undefined" "MultiplyWithRoot" null (`self.Velocidad_0`) null))

(fn `UserConstructionScript`)