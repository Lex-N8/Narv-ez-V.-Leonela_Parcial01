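; BP_Personaje is a character Blueprint that moves by a Velocidad local offset every tick, without sweep, and can spawn BP_Bala bullets.
; SpawnearB creates a bullet at the actor's location and passes it Velocidad, not the separately settable VelocidadBala.
; Setters and helpers for scaling by FloatEditableNum and normalizing ValorNormalizado are defined, but nothing in this graph calls them.
; NormalizeEditable ignores its Valor input.
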(event `self.ReceiveTick`
  (params (DeltaSeconds :type "Float (single-precision)"))
  (`self.K2_AddActorLocalOffset` (`self.Velocidad`)))

(fn `Float Editable`
  (params (Velocidad :type "Vector Structure"))
  (returns (Resultado :type "Vector Structure"))
  ;[1 1 1] Funcion para crear float editable en instancia
  (return (* Velocidad (`self.Float Editable Num`))))

(fn `Normalize Editable`
  (params (Valor :type "Vector Structure"))
  (returns (Resultado :type "Vector Structure"))
  (return (`KismetMathLibrary.Normal` (`self. Valor Normalizado`))))

(fn `SetearVelocidadPj`
  (params (Velocidad :type "Vector Structure"))
  (set `self.Velocidad` Velocidad))

(fn `SetVelocidadBala`
  (params (VelocidadBala :type "Vector Structure"))
  (set `self.Velocidad Bala` VelocidadBala))

(fn `SpawnearB`
  (`|SpawnActorFromClass` "/Game/BP_Bala.BP_Bala_C" (`KismetMathLibrary.MakeTransform` (`self.K2_GetActorLocation`)) "Undefined" "MultiplyWithRoot" null (`self.Velocidad`) null))

(fn `UserConstructionScript`)